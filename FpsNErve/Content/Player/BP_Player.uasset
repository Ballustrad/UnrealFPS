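; Player character Blueprint using Enhanced Input for movement, look, jump, dash and pickup interaction.
; Jump, double jump and a cooldown-limited, input-directed dash use LaunchCharacter; landing restores the double jump and zeroes velocity.
; Interact messages the first overlapping BP_PickUpMaster, while SpawnWeapon drops any current weapon as a pickup, spawns the replacement and attaches it for one WeaponName case.
; A timeline-driven jetpack remains as disconnected, unused logic.
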(event `self.ReceiveBeginPlay`
  ;[1 1 1] Add Mapping
  (`EnhancedInputSubsystemInterface.AddMappingContext` (pcsubsystem `EnhancedInputLocalPlayerSubsystem` (`GameplayStatics.GetPlayerController` 0)) "/Game/Player/Inputs/IMC_Input.IMC_Input" 0 (struct)))

(event `EnhancedInput|/Game/Player/Inputs/IA_Move`
  (params (ActionValue :type "Vector2D Structure") (ElapsedSeconds :type "Float (double-precision)") (TriggeredSeconds :type "Float (double-precision)") (InputAction :type "InputAction Object Reference" :default "/Game/Player/Inputs/IA_Move.IA_Move"))
  (bind (_x _y) (`KismetMathLibrary.BreakVector2D` ActionValue))
  ;[1 1 1] Move
  (:`Triggered`
    (`self.AddMovementInput` (`self.GetActorForwardVector`) _x)
    (`self.AddMovementInput` (`self.GetActorRightVector`) _y)))

(event `EnhancedInput|/Game/Player/Inputs/IA_Look`
  (params (ActionValue :type "Vector2D Structure") (ElapsedSeconds :type "Float (double-precision)") (TriggeredSeconds :type "Float (double-precision)") (InputAction :type "InputAction Object Reference" :default "/Game/Player/Inputs/IA_Look.IA_Look"))
  (bind (_x _y) (`KismetMathLibrary.BreakVector2D` ActionValue))
  ;[1 1 1] Look
  (:`Triggered`
    (`self.AddControllerYawInput` _x)
    (`self.AddControllerPitchInput` _y)))

(event `EnhancedInput|/Game/Player/Inputs/IA_Jump`
  (params (ActionValue :type Boolean) (ElapsedSeconds :type "Float (double-precision)") (TriggeredSeconds :type "Float (double-precision)") (InputAction :type "InputAction Object Reference" :default "/Game/Player/Inputs/IA_Jump.IA_Jump"))
  ;[1 1 1] JetPack et Jump
  (:`Started`
    (if (`NavMovementComponent.IsMovingOnGround` (`self.CharacterMovement`))
      (`self.LaunchCharacter` (0.0 0.0 2000.0) false true)
      (elif (`self.canDoubleJump`)
        (`self.LaunchCharacter` (0.0 0.0 2000.0) false true)
        (set `self.canDoubleJump` false)))))

(event `EnhancedInput|/Game/Player/Inputs/IA_Dash`
  (params (ActionValue :type Boolean) (ElapsedSeconds :type "Float (double-precision)") (TriggeredSeconds :type "Float (double-precision)") (InputAction :type "InputAction Object Reference" :default "/Game/Player/Inputs/IA_Dash.IA_Dash"))
  (bind (_x _y) (`KismetMathLibrary.BreakVector2D` (`|GetInputActionValue`)))
  ;[1 1 1] Dash
  (:`Started`
    (if (`self.CanDash`)
      (`self.LaunchCharacter` (+ (* (+ (* (`self.GetActorForwardVector`) _x) (* (`self.GetActorRightVector`) _y)) 4090.0) (0.0 0.0 512.0)))
      (set `self.CanDash` false)
      (`KismetSystemLibrary.Delay` 5.0)
      (set `self.CanDash` true))))

(event `self.OnLanded`
  (params (Hit :type "HitResult Structure (by ref)"))
  ;[1 1 1] Reset Velocity on landed
  (set `self.canDoubleJump` true)
  (`self.LaunchCharacter` (0.0 0.0 0.0) true true))

(event `EnhancedInput|/Game/Player/Inputs/IA_Interact`
  (params (ActionValue :type Boolean) (ElapsedSeconds :type "Float (double-precision)") (TriggeredSeconds :type "Float (double-precision)") (InputAction :type "InputAction Object Reference" :default "/Game/Player/Inputs/IA_Interact.IA_Interact"))
  (:`Triggered`
    (message `/Game/Interface/BPI_Interact.Interact` (`|GetArrayItem` (`self.GetOverlappingActors` "/Game/Props/PickUps/BP_PickUpMaster.BP_PickUpMaster_C")) null)))

(event `SpawnWeapon`
  (params (WeaponToSpawn :type "/Game/Props/Weapons/BP_WeaponMaster Class Reference"))
  (bind _currentweapon (`self.CurrentWeapon`))
  (`/Engine/EditorBlueprintResources/StandardMacros.IsValid` _currentweapon
    (:`Is Valid`
      (`|SpawnActorFromClass` (`/Game/Props/Weapons/BP_WeaponMaster.PickUpClass` _currentweapon) (`KismetMathLibrary.MakeTransform` (+ (`self.K2_GetActorLocation`) (* (`self.GetActorForwardVector`) (50.0 50.0 0.0)))) "Undefined" "MultiplyWithRoot" null null)
      (`self.K2_DestroyActor` _currentweapon))
    (:`Is Not Valid`
      _))
  (bind _returnvalue (`|SpawnActorFromClass` WeaponToSpawn (`KismetMathLibrary.MakeTransform` (0.0 0.0 0.0)) "Undefined" "MultiplyWithRoot" null null))
  (bind _output_get (set `self.CurrentWeapon` _returnvalue))
  (switch `/Game/Props/Weapons/Enum_WeaponName` (`/Game/Props/Weapons/BP_WeaponMaster.WeaponName` _output_get)
    (:`NewEnumerator1`
      (`self.K2_AttachToComponent` _output_get (`self.ParentTransform`) "None" "KeepRelative" "KeepRelative" "KeepRelative" true))))

(fn `UserConstructionScript`)